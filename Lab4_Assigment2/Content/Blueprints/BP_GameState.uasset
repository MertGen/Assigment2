(event Custom|Blue%20Won
  (bind _blue_won_bool (Variables|Default|GetBlue%20Won%20Bool))
  (for _array_element (Variables|Default|GetPlayerArray)
    (bind _asnet_player_state (Utilities|Casting|CastToNetPlayerState _array_element))
    (switch Utilities|FlowControl|Switch|SwitchonEPlayerTeam (.teamid (Variables|/Script/Lab4_Assigment2.NetPlayerState|GetData _asnet_player_state))
      (:TEAM_Blue
        (if _blue_won_bool
          (Default|OnPlayerWon (.AsBP%20Net%20Avatar (Utilities|Casting|CastToBP_NetAvatar (Variables|/Script/Engine.PlayerState|GetPawnPrivate _asnet_player_state))))
          (else
            (Default|OnPlayerLost (.AsBP%20Net%20Avatar (Utilities|Casting|CastToBP_NetAvatar (Variables|/Script/Engine.PlayerState|GetPawnPrivate _asnet_player_state)))))))
      (:TEAM_Red
        (if _blue_won_bool
          (Default|OnPlayerLost (.AsBP%20Net%20Avatar (Utilities|Casting|CastToBP_NetAvatar (Variables|/Script/Engine.PlayerState|GetPawnPrivate _asnet_player_state))))
          (else
            (Default|OnPlayerWon (.AsBP%20Net%20Avatar (Utilities|Casting|CastToBP_NetAvatar (Variables|/Script/Engine.PlayerState|GetPawnPrivate _asnet_player_state)))))))))
  (CallFunction|ShowResultMessage))

(event EventBeginPlay)

(event EventTick
  (params (DeltaSeconds :type Float%20%28single-precision%29)))

(event EventOnVictory
  (bind _blue_won_bool (Variables|Default|GetBlue%20Won%20Bool))
  (for _array_element (Variables|Default|GetPlayerArray)
    (bind _asnet_player_state (Utilities|Casting|CastToNetPlayerState _array_element))
    (switch Utilities|FlowControl|Switch|SwitchonEPlayerTeam (.teamid (Variables|/Script/Lab4_Assigment2.NetPlayerState|GetData _asnet_player_state))
      (:TEAM_Blue
        (if _blue_won_bool
          (Default|OnPlayerWon (.AsBP%20Net%20Avatar (Utilities|Casting|CastToBP_NetAvatar (Variables|/Script/Engine.PlayerState|GetPawnPrivate _asnet_player_state))))
          (else
            (Default|OnPlayerLost (.AsBP%20Net%20Avatar (Utilities|Casting|CastToBP_NetAvatar (Variables|/Script/Engine.PlayerState|GetPawnPrivate _asnet_player_state)))))))
      (:TEAM_Red
        (if _blue_won_bool
          (Default|OnPlayerLost (.AsBP%20Net%20Avatar (Utilities|Casting|CastToBP_NetAvatar (Variables|/Script/Engine.PlayerState|GetPawnPrivate _asnet_player_state))))
          (else
            (Default|OnPlayerWon (.AsBP%20Net%20Avatar (Utilities|Casting|CastToBP_NetAvatar (Variables|/Script/Engine.PlayerState|GetPawnPrivate _asnet_player_state)))))))))
  (CallFunction|ShowResultMessage))

(event EventOnRestart
  (Widget|RemovefromParent (Variables|Default|GetMessage%20Widget)))

(fn ConstructionScript)

(fn ShowResultMessage
  (bind _returnvalue (Class|NetGameState|GetPlayerStatebyIndex (Variables|Default|GetWinningPlayer)))
  (bind _returnvalue_2 (UserInterface|CreateWidget "/Game/Blueprints/UMG/W_GameResults.W_GameResults_C" 0 (select (Utilities|Enum|Equal(Enum) (.teamid (Variables|/Script/Lab4_Assigment2.NetPlayerState|GetData (.AsNet%20Player%20State (Utilities|Casting|CastToNetPlayerState (Variables|/Script/Engine.Controller|GetPlayerState (Game|GetPlayerController 0)))))) "TEAM_Blue") "YOU LOSE" (Utilities|Text|FormatText "{Name} WINS!" (.Nickname (Utilities|Struct|BreakSPlayerInfo (Variables|/Script/Lab4_Assigment2.NetPlayerState|GetData _returnvalue)))))))
  (bind _output_get (Variables|Default|SetMessage%20Widget _returnvalue_2))
  (UserInterface|Viewport|AddtoViewport _output_get 0))